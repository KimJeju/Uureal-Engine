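; LIGHT_BP is an interactive spotlight actor that the player switches on and off with the F key while nearby.
; A trigger volume enables input for player controller 0 and toggles the helpful text on begin overlap, then reverses both on end overlap, without filtering the overlapping actor.
; The construction script applies the configurable light color and initial visibility to the spotlight.
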(event `self.Tirrger.OnComponentBeginOverlap`
  (params (OverlappedComponent :type "PrimitiveComponent Object Reference") (OtherActor :type "Actor Object Reference") (OtherComp :type "PrimitiveComponent Object Reference") (OtherBodyIndex :type Integer) (bFromSweep :type Boolean) (SweepResult :type "HitResult Structure (by ref)"))
  ;[0.9819 1 0.2337] Trigger Volume 에 접근하면 입력을 허가하고 HelpFul Text를 보여줌, 떠나면 그와  반대
  (`self.EnableInput` (`GameplayStatics.GetPlayerController` 0))
  (`SceneComponent.ToggleVisibility` (`self.HelpfulText`) false :!label _label))

(event `self.Tirrger.OnComponentEndOverlap`
  (params (OverlappedComponent :type "PrimitiveComponent Object Reference") (OtherActor :type "Actor Object Reference") (OtherComp :type "PrimitiveComponent Object Reference") (OtherBodyIndex :type Integer))
  ;[0.9819 1 0.2337] Trigger Volume 에 접근하면 입력을 허가하고 HelpFul Text를 보여줌, 떠나면 그와  반대
  (`self.DisableInput` (`GameplayStatics.GetPlayerController` 0))
  (goto _label))

(event `Key|F`
  (params (Key :type "Key Structure"))
  ;[0.2262 0.1594 1] F 를 눌러 라이트 제어
  (:`Pressed`
    (`SceneComponent.ToggleVisibility` (`self.SpotLight`) false)))

(fn `UserConstructionScript`
  (bind _spotlight (`self.SpotLight`))
  (`LightComponent.SetLightColor` _spotlight (`self.Light Color`) true)
  (`SceneComponent.SetVisibility` _spotlight (`self.Visbililty Setting`) false))